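; Camera controller that drives the MainCamera pawn with movement, rotation and zoom, caching it and CityGameState on BeginPlay.
; Holding Pan opens gates that let mouse axes rotate yaw and clamped pitch, while ResetPan levels the pitch.
; Zoom actions adjust or reset spring arm length, which MoveSpeedCalc turns into a clamped move speed.
; MoveX and MoveY offset the pawn along its own axes, with sideways movement forcing a fixed height.
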(event EventBeginPlay
  ;[1 1 1] Camera Functions
  ;;[1 1 1] BeginPlay
  (Utilities|FlowControl|Sequence
    (:then_0
      (Utilities|CastReferences))))

(event Input|ActionEvents|InputActionZoomIn
  (params (Key :type Key%20Structure :default "None"))
  (bind _camerapawnref (Variables|Default|GetCameraPawnRef))
  (bind _springarm (Variables|/Game/Bridgebuild/Blueprints/MainCamera.MainCamera_C|GetSpringArm _camerapawnref))
  ;[1 1 1] Camera Functions
  ;;[1 1 1] Zooming in and Out function
  (:Pressed
    (Variables|/Script/Engine.SpringArmComponent|SetTargetArmLength _springarm (Math|Float|Clamp(Float) (- (Variables|/Script/Engine.SpringArmComponent|GetTargetArmLength _springarm) (Variables|Default|GetZoomSensitivity)) 5e+02 (Variables|Default|GetMaxArmDistance)))))

(event Input|ActionEvents|InputActionZoomOut
  (params (Key :type Key%20Structure :default "None"))
  (bind _camerapawnref (Variables|Default|GetCameraPawnRef))
  (bind _springarm (Variables|/Game/Bridgebuild/Blueprints/MainCamera.MainCamera_C|GetSpringArm _camerapawnref))
  ;[1 1 1] Camera Functions
  ;;[1 1 1] Zooming in and Out function
  (:Pressed
    (Variables|/Script/Engine.SpringArmComponent|SetTargetArmLength _springarm (Math|Float|Clamp(Float) (+ (Variables|/Script/Engine.SpringArmComponent|GetTargetArmLength _springarm) (Variables|Default|GetZoomSensitivity)) 5e+02 (Variables|Default|GetMaxArmDistance)))))

(event Input|ActionEvents|InputActionZoomReset
  (params (Key :type Key%20Structure :default "None"))
  ;[1 1 1] Camera Functions
  ;;[1 1 1] Reset Zoom Command
  (:Pressed
    (Variables|/Script/Engine.SpringArmComponent|SetTargetArmLength (Variables|/Game/Bridgebuild/Blueprints/MainCamera.MainCamera_C|GetSpringArm (Variables|Default|GetCameraPawnRef)) 1.5e+03)))

(event Input|ActionEvents|InputActionPan
  (params (Key :type Key%20Structure :default "None"))
  (bind _camerapawnref (Variables|Default|GetCameraPawnRef))
  (bind _returnvalue (Transformation|GetActorRotation _camerapawnref))
  (bind (_roll _pitch _yaw) (Math|Rotator|BreakRotator _returnvalue))
  ;[1 1 1] Camera Functions
  ;;[1 1 1] Pan Y Axis
  (:Pressed
    (Variables|Default|SetDisableCamNav false)
    (Utilities|FlowControl|Gate true) ; enters at Open
  )
  (:Released
    (Variables|Default|SetDisableCamNav false)
    (Utilities|FlowControl|Gate true) ; enters at Close
  ))

(event Input|ActionEvents|InputActionPan
  (params (Key :type Key%20Structure :default "None"))
  (bind _camerapawnref (Variables|Default|GetCameraPawnRef))
  (bind _returnvalue (Transformation|GetActorRotation _camerapawnref))
  (bind (_roll _pitch _yaw) (Math|Rotator|BreakRotator _returnvalue))
  ;[1 1 1] Camera Functions
  ;;[1 1 1] Pan X Axis
  (:Pressed
    (Variables|Default|SetDisableCamNav true)
    (Utilities|FlowControl|Gate true) ; enters at Open
  )
  (:Released
    (Variables|Default|SetDisableCamNav false)
    (Utilities|FlowControl|Gate true) ; enters at Close
  ))

(event Input|ActionEvents|InputActionResetPan
  (params (Key :type Key%20Structure :default "None"))
  (bind _camerapawnref (Variables|Default|GetCameraPawnRef))
  (bind _returnvalue (Transformation|GetActorRotation _camerapawnref))
  (bind (_roll _pitch _yaw) (Math|Rotator|BreakRotator _returnvalue))
  ;[1 1 1] Camera Functions
  ;;[1 1 1] ResetPan
  (:Pressed
    (Transformation|SetActorRotation _camerapawnref (Math|Rotator|MakeRotator _roll 0.0 _yaw))))

(event Input|AxisEvents|InputAxisMoveForward
  (params (AxisValue :type Float%20%28single-precision%29))
  ;[1 1 1] Camera Functions
  ;;[1 1 1] MoveX
  (if (not (Variables|Default|GetDisableCamNav))
    (Transformation|SetActorTransform (Variables|Default|GetCameraPawnRef) (Utilities|MoveX (CallFunction|MoveSpeedCalc) 1.0 (Variables|Default|GetCameraPawnRef) AxisValue))))

(event Input|AxisEvents|InputAxisMoveRight
  (params (AxisValue :type Float%20%28single-precision%29))
  (bind _movesensitivity (CallFunction|MoveSpeedCalc))
  (bind _camerapawnref (Variables|Default|GetCameraPawnRef))
  (bind _transform (Utilities|MoveY _movesensitivity AxisValue 1.0 _camerapawnref))
  (bind (_location _rotation _scale) (Math|Transform|BreakTransform _transform))
  (bind (_x _y) (Math|Vector|BreakVector _location))
  ;[1 1 1] Camera Functions
  ;;[1 1 1] MoveY
  (if (not (Variables|Default|GetDisableCamNav))
    (Transformation|SetActorTransform (Variables|Default|GetCameraPawnRef) (Math|Transform|MakeTransform (Math|Vector|MakeVector _x _y 2e+02) _rotation _scale))))

(event Input|MouseEvents|MouseX
  (params (AxisValue :type Float%20%28single-precision%29))
  (bind _camerapawnref (Variables|Default|GetCameraPawnRef))
  (bind _returnvalue (Transformation|GetActorRotation _camerapawnref))
  (bind (_roll _pitch _yaw) (Math|Rotator|BreakRotator _returnvalue))
  ;[1 1 1] Camera Functions
  ;;[1 1 1] Pan X Axis
  (Utilities|FlowControl|Gate true
    (:Exit
      (Transformation|SetActorRotation (Variables|Default|GetCameraPawnRef) (Math|Rotator|MakeRotator _roll _pitch (+ _yaw (* (Variables|Default|GetPanSensitivity) AxisValue)))))))

(event Input|MouseEvents|MouseY
  (params (AxisValue :type Float%20%28single-precision%29))
  (bind _camerapawnref (Variables|Default|GetCameraPawnRef))
  (bind _returnvalue (Transformation|GetActorRotation _camerapawnref))
  (bind (_roll _pitch _yaw) (Math|Rotator|BreakRotator _returnvalue))
  ;[1 1 1] Camera Functions
  ;;[1 1 1] Pan Y Axis
  (Utilities|FlowControl|Gate true
    (:Exit
      (Transformation|SetActorRotation (Variables|Default|GetCameraPawnRef) (Math|Rotator|MakeRotator _roll (Math|Float|Clamp(Float) (+ _pitch (* (Variables|Default|GetPanSensitivity) AxisValue)) -15.0 5e+01) _yaw)))))

(fn ConstructionScript)

(fn MovetoHitLocation
  (params (Hit :type Hit%20Result%20Structure)))

(fn MoveSpeedCalc
  (return (Math|Float|Clamp(Float) (/ (Variables|/Script/Engine.SpringArmComponent|GetTargetArmLength (Variables|/Game/Bridgebuild/Blueprints/MainCamera.MainCamera_C|GetSpringArm (Variables|Default|GetCameraPawnRef))) 1e+02) 5.0 2e+01)))